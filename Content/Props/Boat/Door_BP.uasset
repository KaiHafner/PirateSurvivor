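; Boat door prop whose bars the player breaks by repeatedly pressing E.
; Overlap with the third-person character toggles input and a prompt widget, which appears only while the bars are intact.
; Each press plays a metal clank and advances a counter that triggers the break at four, despite a comment claiming 15 presses.
; Breaking hides the bars and widget, disables bar collision, and adds a non-colliding replacement mesh at runtime.
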(event `self.ReceiveActorBeginOverlap`
  (params (OtherActor :type "Actor Object Reference"))
  ;[1 1 1] Overlap checks
  (cast `/Game/ThirdPerson/Blueprints/BP_ThirdPersonCharacter` OtherActor)
  (`self.EnableInput` (`GameplayStatics.GetPlayerController` 0))
  (if (not (`self.broken`))
    (`SceneComponent.SetVisibility` (`self.Widget`) true false)))

(event `self.ReceiveActorEndOverlap`
  (params (OtherActor :type "Actor Object Reference"))
  ;[1 1 1] Overlap checks
  (cast `/Game/ThirdPerson/Blueprints/BP_ThirdPersonCharacter` OtherActor)
  (`self.DisableInput` (`GameplayStatics.GetPlayerController` 0))
  (`SceneComponent.SetVisibility` (`self.Widget`) false false))

(event `Key|E`
  (params (Key :type "Key Structure"))
  ;[1 1 1] Player spams the E key 15 times untill the bars break.
  (:`Pressed`
    (if (not (`self.broken`))
      (`GameplayStatics.PlaySound2D` "/Game/audio/243260-metal_clank_heavy-05.243260-metal_clank_heavy-05" 1.0 1.0 0.0 null null)
      (if (== (`self.PressedE`) 4)
        (bind _returnvalue (`AddComponent|NODE_AddStaticMeshComponent-0`))
        (`PrimitiveComponent.SetCollisionEnabled` _returnvalue "NoCollision")
        (`PrimitiveComponent.SetCollisionEnabled` (`self.bars`) "NoCollision")
        (`SceneComponent.SetVisibility` _returnvalue true false)
        (`SceneComponent.SetVisibility` (`self.bars`) false false)
        (`SceneComponent.SetVisibility` (`self.Widget`) false false)
        (set `self.broken` true)
        (else
          (set `self.PressedE` (+ (`self.PressedE`) 1)))))))

(fn `UserConstructionScript`)