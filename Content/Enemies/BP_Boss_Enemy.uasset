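; Boss enemy character that chases the player on sight, attacks in melee and returns the game to LevelSelect when killed.
; Pawn sensing triggers an AI move, then a montage and sphere overlap at an arrow damages Player-tagged actors.
; Damage passes a DoOnce cooldown, updates the health widget and plays block-react or death montages.
; Hair, legs, chest and beard follow the main mesh through leader pose.
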(event `self.ReceiveTick`
  (params (DeltaSeconds :type "Float (single-precision)"))
  (if (not (`self.isPlayerVisible`))
    (`MovementComponent.StopMovementImmediately` (`self.CharacterMovement`))))

(event `self.PawnSensing.OnSeePawn`
  (params (Pawn :type "Pawn Object Reference"))
  (set `self.isPlayerVisible` true)
  (`self.FollowPlayer`))

(event `FollowPlayer`
  (if (`self.isPlayerVisible`)
    (if (> (`self.HealthBoss`) 0.0)
      (`|AIMoveTo` self (0.0 0.0 0.0) (`GameplayStatics.GetPlayerCharacter` 0) 70.0
        (:`OnSuccess`
          (if (`self.canAttack`)
            (set `self.canAttack` false)
            (bind _returnvalue (`self.PlayAnimMontage` "/Game/BodyTypes/Anims/AniMont/SK_Head_0_Anim_SK_Rig_Standing_Melee_Attack_Horizontal_Montage.SK_Head_0_Anim_SK_Rig_Standing_Melee_Attack_Horizontal_Montage"))
            (bind _outactors (`KismetSystemLibrary.SphereOverlapActors` (`SceneComponent.K2_GetComponentLocation` (`self.Arrow1`)) 10.0 (`self.Object Types`)))
            (for _array_element _outactors
              (if (`self.ActorHasTag` _array_element "Player")
                (`GameplayStatics.ApplyDamage` _array_element 20.0)
                (`KismetSystemLibrary.Delay` _returnvalue :!label _label)
                (set `self.canAttack` true)))
            (goto _label))))
      (else
        (set `self.isPlayerVisible` false :!label _label_2)))
    (else
      (goto _label_2))))

(event `self.ReceiveAnyDamage`
  (params (Damage :type "Float (single-precision)") (DamageType :type "DamageType Object Reference") (InstigatedBy :type "Controller Object Reference") (DamageCauser :type "Actor Object Reference"))
  (`KismetSystemLibrary.PrintString` (`KismetStringLibrary.Conv_DoubleToString` (`self.HealthBoss`)))
  (`/Engine/EditorBlueprintResources/StandardMacros.DoOnce` false :!label _label
    (:`Completed`
      (bind _output_get (set `self.HealthBoss` (- (`self.HealthBoss`) Damage)))
      (set `/Game/UIs/WP_EnemyBoss.HealthBoss` _output_get (`self.HealthREF`))
      (if (<= _output_get 0.0)
        (`MovementComponent.StopMovementImmediately` (`self.CharacterMovement`))
        (`ActorComponent.K2_DestroyComponent` (`self.Widget`))
        (`ActorComponent.K2_DestroyComponent` (`self.CapsuleComponent`))
        (bind _returnvalue (`self.PlayAnimMontage` "/Game/BodyTypes/Anims/AniMont/SK_Head_0_Anim_SK_Rig_Death_Montage.SK_Head_0_Anim_SK_Rig_Death_Montage"))
        (`KismetSystemLibrary.Delay` _returnvalue)
        (`self.K2_DestroyActor`)
        (`self.On Destroyed`)
        (`GameplayStatics.OpenLevel` "LevelSelect")
        (else
          (`self.PlayAnimMontage` "/Game/BodyTypes/Anims/AniMont/SK_Head_0_Anim_SK_Rig_Standing_Block_React_Montage.SK_Head_0_Anim_SK_Rig_Standing_Block_React_Montage")
          (`KismetSystemLibrary.Delay` 0.2)
          (goto _label :!via `Reset`))))))

(event `self.ReceiveBeginPlay`
  (bind _aswp_enemy_boss (cast `/Game/UIs/WP_EnemyBoss` (`WidgetComponent.GetUserWidgetObject` (`self.Widget`))))
  (set `self.HealthREF` _aswp_enemy_boss))

(fn `UserConstructionScript`
  (`SkinnedMeshComponent.SetLeaderPoseComponent` (`self.Hair`) (`self.Mesh`) false false)
  (`SkinnedMeshComponent.SetLeaderPoseComponent` (`self.Legs`) (`self.Mesh`) false false)
  (`SkinnedMeshComponent.SetLeaderPoseComponent` (`self.Chest`) (`self.Mesh`) false false)
  (`SkinnedMeshComponent.SetLeaderPoseComponent` (`self.Beard`) (`self.Mesh`) false false))